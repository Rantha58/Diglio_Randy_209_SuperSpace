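; BP_Asteroide is an asteroid obstacle that ends the game when the player's spaceship touches it.
; When BP_SpaceShip overlaps its Sphere_Tigger component, it adds the Lose_UI widget to the viewport, pauses the game and destroys itself.
; Tick sets the relative rotation to random values scaled by delta time, replacing it each frame rather than accumulating, so it jitters instead of spinning.
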(event OnComponentBeginOverlap(Sphere_Tigger)
  (params (OverlappedComponent :type Primitive%20Component%20Object%20Reference) (OtherActor :type Actor%20Object%20Reference) (OtherComp :type Primitive%20Component%20Object%20Reference) (OtherBodyIndex :type Integer) (bFromSweep :type Boolean) (SweepResult :type Hit%20Result%20Structure%20%28by%20ref%29))
  (Utilities|Casting|CastToBP_SpaceShip OtherActor)
  (bind _returnvalue (UserInterface|CreateWidget "/Game/Proto/Interface/Lose_UI.Lose_UI_C"))
  (UserInterface|Viewport|AddtoViewport _returnvalue 0)
  (Game|SetGamePaused true)
  (Actor|DestroyActor))

(event EventTick
  (params (DeltaSeconds :type Float%20%28single-precision%29))
  (bind _returnvalue (Math|Random|RandomFloat))
  (Transformation|SetActorRelativeRotation (Math|Rotator|MakeRotator (* DeltaSeconds _returnvalue) (* DeltaSeconds _returnvalue) (* DeltaSeconds _returnvalue))))

(fn ConstructionScript)