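; Prototype spaceship that advances continuously and is steered by 2D mouse input.
; Each Tick adds a world offset: scaled Mouse2D axes drive X and Z, while the forward vector's X component, scaled by speed and delta time, drives Y.
; The mouse terms are not scaled by delta time.
; BeginPlay caches the mesh position, used only by disconnected leftover nodes for screen-centre-relative cursor positioning.
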(event EventBeginPlay
  (Variables|Default|SetOriginalShipPosition (Transformation|GetWorldLocation (Variables|Default|GetStaticMesh))))

(event EventTick
  (params (DeltaSeconds :type Float%20%28single-precision%29))
  (bind _returnvalue (Settings|GetGameUserSettings))
  (bind _output_get (Variables|Default|Setforward 1.2e+03))
  (Transformation|AddActorWorldOffset (Math|Vector|MakeVector (* (.x (stale Input|MouseEvents|Mouse2D AxisValue)) -1e+01) (.X (Math|Vector|BreakVector (* (* (Transformation|GetActorForwardVector) _output_get) DeltaSeconds))) (* (.y (stale Input|MouseEvents|Mouse2D AxisValue)) 2e+01))))

(event Input|MouseEvents|Mouse2D
  (params (AxisValue :type Vector :default "0, 0, 0")))

(fn ConstructionScript)